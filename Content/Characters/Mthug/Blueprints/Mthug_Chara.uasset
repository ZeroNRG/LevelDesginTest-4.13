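; Mthug character Blueprint that sets its active weapon mesh, binds that mesh to the body's pose and carries a prototype ledge-climbing system.
; A sphere overlap toggles CanTrace, ignoring DystopianCharacterBase actors on entry, and the ClimbingLedgeBI event stores climb state and restores walking movement.
; The sphere-trace logic that finds walls and ledges, snaps the capsule into a hang and notifies the AnimInstance is disconnected, so it never runs.
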(event OnComponentBeginOverlap(Sphere)
  (params (OverlappedComponent :type Primitive%20Component%20Object%20Reference) (OtherActor :type Actor%20Object%20Reference) (OtherComp :type Primitive%20Component%20Object%20Reference) (OtherBodyIndex :type Integer) (bFromSweep :type Boolean) (SweepResult :type Hit%20Result%20Structure%20%28by%20ref%29))
  (Utilities|Casting|CastToDystopianCharacterBase (Components|GetOwner OtherComp)
    (:CastFailed
      (Variables|Default|SetCanTrace true))))

(event OnComponentEndOverlap(Sphere)
  (params (OverlappedComponent :type Primitive%20Component%20Object%20Reference) (OtherActor :type Actor%20Object%20Reference) (OtherComp :type Primitive%20Component%20Object%20Reference) (OtherBodyIndex :type Integer))
  (Variables|Default|SetCanTrace false))

(event EventBeginPlay
  (Variables|Default|SetActiveWeaponMesh (Variables|Default|GetWeapon_Mesh)))

(event Collision|EventActorBeginOverlap
  (params (OtherActor :type Actor%20Object%20Reference)))

(event EventTick
  (params (DeltaSeconds :type Float%20%28single-precision%29)))

(event EventClimbingLedgeBI
  (params (IsClimbing :type Boolean))
  (Variables|Default|SetIsClimbingLedge IsClimbing)
  (Pawn|Components|CharacterMovement|SetMovementMode (Variables|Character|GetCharacterMovement) "MOVE_Walking" 0)
  (Components|Activation|Activate (Variables|Character|GetCharacterMovement) false))

(fn ConstructionScript
  (bind _weapon_mesh (Variables|Default|GetWeapon_Mesh))
  (Utilities|IsValid _weapon_mesh
    (:Is%20Valid
      (Class|SkinnedMeshComponent|SetMasterPoseComponent _weapon_mesh (Variables|Character|GetMesh)))))