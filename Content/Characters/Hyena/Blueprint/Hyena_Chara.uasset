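; Hyena character Blueprint with a dropship landing, a trace-based jump and unfinished ledge climbing.
; When ShuttleSpawn is set, the first landing plays a drop animation with movement paused, then restores the animation Blueprint.
; NumPad 2 launches it vertically if a trace above JumpBox is clear and one below hits.
; Sphere-trace ledge grab and climb logic is disconnected; the overlap-driven CanTrace check on Tick does nothing.
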(event OnComponentBeginOverlap(Sphere)
  (params (OverlappedComponent :type Primitive%20Component%20Object%20Reference) (OtherActor :type Actor%20Object%20Reference) (OtherComp :type Primitive%20Component%20Object%20Reference) (OtherBodyIndex :type Integer) (bFromSweep :type Boolean) (SweepResult :type Hit%20Result%20Structure%20%28by%20ref%29))
  (Utilities|Casting|CastToDystopianCharacterBase (Components|GetOwner OtherComp)
    (:CastFailed
      (Variables|Default|SetCanTrace true))))

(event OnComponentBeginOverlap(Box_0)
  (params (OverlappedComponent :type Primitive%20Component%20Object%20Reference) (OtherActor :type Actor%20Object%20Reference) (OtherComp :type Primitive%20Component%20Object%20Reference) (OtherBodyIndex :type Integer) (bFromSweep :type Boolean) (SweepResult :type Hit%20Result%20Structure%20%28by%20ref%29)))

(event OnComponentEndOverlap(Sphere)
  (params (OverlappedComponent :type Primitive%20Component%20Object%20Reference) (OtherActor :type Actor%20Object%20Reference) (OtherComp :type Primitive%20Component%20Object%20Reference) (OtherBodyIndex :type Integer))
  (Variables|Default|SetCanTrace false))

(event EventBeginPlay)

(event EventTick
  (params (DeltaSeconds :type Float%20%28single-precision%29))
  (if (Variables|Default|GetCanTrace)
    _))

(event EventClimbingLedgeBI
  (params (IsClimbing :type Boolean))
  (Variables|Default|SetIsClimbingLedge IsClimbing)
  (Pawn|Components|CharacterMovement|SetMovementMode (Variables|Character|GetCharacterMovement) "MOVE_Walking" 0)
  (Components|Activation|Activate (Variables|Character|GetCharacterMovement) false))

(event EventOnLanded
  (params (Hit :type Hit%20Result%20Structure%20%28by%20ref%29))
  (if (Variables|Default|GetShuttleSpawn)
    (Utilities|FlowControl|DoOnce false
      (:Completed
        (Components|Animation|PlayAnimation (Variables|Character|GetMesh) "/Game/Characters/Hyena/Animation/Hyena_Dropship_DropShipLand.Hyena_Dropship_DropShipLand" false)
        (Components|Activation|SetActive (Variables|Character|GetCharacterMovement) false false)
        (Utilities|FlowControl|Delay 1.7)
        (Components|Animation|SetAnimationMode (Variables|Character|GetMesh) "AnimationBlueprint")
        (Components|Activation|SetActive (Variables|Character|GetCharacterMovement) true false)))))

(event Input|KeyboardEvents|NumPadTwo
  (params (Key :type Key%20Structure :default "AnyKey"))
  (bind _jumpbox (Variables|Default|GetJumpBox))
  (bind _returnvalue (Transformation|GetWorldLocation _jumpbox))
  (bind _returnvalue_2 (Transformation|GetWorldLocation _jumpbox))
  (bind (_x _y _z) (Math|Vector|BreakVector _returnvalue))
  (bind (_x_2 _y_2 _z_2) (Math|Vector|BreakVector _returnvalue_2))
  (:Pressed
    (bind _returnvalue_3 (Collision|LineTraceByChannel _returnvalue (Math|Vector|MakeVector _x _y (- _z -1041.0)) "TraceTypeQuery1" false 0 "Persistent"))
    (if (not _returnvalue_3)
      (bind _outhit (Collision|LineTraceByChannel _returnvalue_2 (Math|Vector|MakeVector _x_2 _y_2 (- _z_2 1041.0)) "TraceTypeQuery1" false 0 "Persistent"))
      (if (.bBlockingHit (Collision|BreakHitResult _outhit))
        (Character|LaunchCharacter (Math|Vector|MakeVector 0.0 0.0 (- (- (.Z (Math|Vector|BreakVector (.ImpactPoint (Collision|BreakHitResult _outhit)))) (.Z (Math|Vector|BreakVector (Transformation|GetActorLocation)))) (Components|Movement|GetGravityZ (Variables|Character|GetCharacterMovement)))) false false)))))

(fn ConstructionScript)