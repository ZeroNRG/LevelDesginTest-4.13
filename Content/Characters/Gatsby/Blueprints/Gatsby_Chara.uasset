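; Player character Blueprint for Gatsby, a shooter hero with walk/run, aiming, melee and switchable first- and third-person views.
; Sniper and shotgun selection loads stats, mesh and handedness from a data table via WeaponVariables.
; Firing is rate-gated hitscan: randomly spread camera traces, repeated per BurstCount, draw beam effects, damage DystopianCharacterBase hits and trigger weapon animations.
; Cellphone and save inputs open the in-game menu; debug keys alter health and damage.
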(event Custom|IsShooting
  ;[1 1 1] Run
)

(event Custom|Close_Cell
  (Variables|Default|SetWeaponSwitch false)
  (Variables|Default|SetCanShoot false)
  (Utilities|FlowControl|Delay 0.2)
  (Variables|Default|SetCellphoneEquipped? false)
  (Variables|Default|SetWeaponSwitch false)
  (Variables|Default|SetCanShoot true))

(event Input|ActionEvents|InputActionRun
  (params (Key :type Key%20Structure :default "AnyKey"))
  (bind _charactermovement (Variables|Character|GetCharacterMovement))
  (bind _charactermovement_2 (Variables|Character|GetCharacterMovement))
  (bind _charactermovement_3 (Variables|Character|GetCharacterMovement))
  ;[1 1 1] Run
  (:Pressed
    (if (Variables|Default|GetAiming?)
      (Variables|/Script/Engine.CharacterMovementComponent|SetMaxWalkSpeed (Variables|Character|GetCharacterMovement) (Variables|Default|GetDefaultRunSpeed))
      (Variables|/Script/Engine.CharacterMovementComponent|SetbUseControllerDesiredRotation _charactermovement true)
      (Variables|/Script/Engine.CharacterMovementComponent|SetbOrientRotationToMovement _charactermovement false)
      (else
        (Variables|/Script/Engine.CharacterMovementComponent|SetMaxWalkSpeed (Variables|Character|GetCharacterMovement) (Variables|Default|GetDefaultRunSpeed))
        (Variables|/Script/Engine.CharacterMovementComponent|SetbUseControllerDesiredRotation _charactermovement_3 false)
        (Variables|/Script/Engine.CharacterMovementComponent|SetbOrientRotationToMovement _charactermovement_3 true))))
  (:Released
    (Variables|/Script/Engine.CharacterMovementComponent|SetMaxWalkSpeed _charactermovement_2 (Variables|Default|GetDefaultWalkSpeed))
    (Variables|/Script/Engine.CharacterMovementComponent|SetbOrientRotationToMovement _charactermovement_2 false)
    (Variables|/Script/Engine.CharacterMovementComponent|SetbUseControllerDesiredRotation _charactermovement_2 true)))

(event Input|ActionEvents|InputActionSelectSniper
  (params (Key :type Key%20Structure :default "AnyKey"))
  ;[1 1 1] SwitchWeapon
  (:Pressed
    (bind _returnvalue (Utilities|GetDataTableRow "/Game/Characters/Weapons/Gatsby_WeaponTable.Gatsby_WeaponTable" "Sniper")
      (:then
        (CallFunction|WeaponVariables _returnvalue)
        (Transformation|SetRelativeLocation (Variables|Default|GetSpringArm) "0, 0,-10.000000" false false)))))

(event Input|ActionEvents|InputActionShotgunSelect
  (params (Key :type Key%20Structure :default "AnyKey"))
  ;[1 1 1] SwitchWeapon
  (:Pressed
    (bind _returnvalue (Utilities|GetDataTableRow "/Game/Characters/Weapons/Gatsby_WeaponTable.Gatsby_WeaponTable" "Shotgun")
      (:then
        (CallFunction|WeaponVariables _returnvalue)
        (Transformation|SetRelativeLocation (Variables|Default|GetSpringArm) "0, 0,40.000000" false false)))))

(event Input|ActionEvents|InputActionFireButton
  (params (Key :type Key%20Structure :default "AnyKey"))
  (bind _returnvalue (Game|GetPlayerCameraManager 0))
  (bind _weaponspread (Variables|Default|GetWeaponSpread))
  (bind _returnvalue_2 (Transformation|GetActorRotation _returnvalue))
  (bind _returnvalue_3 (Transformation|GetActorLocation _returnvalue))
  (bind _returnvalue_4 (* _weaponspread -1.0))
  (bind (_roll _pitch _yaw) (Math|Rotator|BreakRotator _returnvalue_2))
  ;[1 1 1] BulletLogic
  (:Pressed
    (Utilities|FlowControl|Gate false :!label _label
      (:Exit
        (Utilities|FlowControl|Sequence
          (:then_0
            (goto _label Close))
          (:then_1
            (Utilities|FlowControl|DoN (Variables|Default|GetBurstCount) :!label _label_2
              (:Exit
                (Utilities|FlowControl|Sequence
                  (:then_0
                    (bind (_outhit _returnvalue_5) (Collision|LineTraceByChannel _returnvalue_3 (+ (* (Math|Vector|GetForwardVector (Math|Rotator|MakeRotator _roll (+ _pitch (Math|Random|RandomFloatinRange _returnvalue_4 _weaponspread)) (+ _yaw (Math|Random|RandomFloatinRange _returnvalue_4 _weaponspread)))) (Variables|Default|GetAttackRange)) _returnvalue_3) "TraceTypeQuery1" true 0 "None"))
                    (Utilities|FlowControl|Sequence
                      (:then_0
                        (bind _returnvalue_6 (Effects|SpawnEmitteratLocation "/Game/Vehicals/Mecha/HumptyDumpty/Projectiles/RailGun_Beam.RailGun_Beam" (Transformation|GetSocketLocation (Variables|Default|GetWeapon_R) "Barrel") "0, 0,0.000000"))
                        (if _returnvalue_5
                          (Effects|Components|ParticleSystem|SetVectorParameter _returnvalue_6 "TrailBeamEnd" (.ImpactPoint (Collision|BreakHitResult _outhit)))
                          (else
                            (Effects|Components|ParticleSystem|SetVectorParameter _returnvalue_6 "TrailBeamEnd" (.TraceEnd (Collision|BreakHitResult _outhit))))))
                      (:then_1
                        (Utilities|FlowControl|DoOnce false :!label _label_3
                          (:Completed
                            (if (Variables|Default|GetLeftHanded?)
                              (bind _returnvalue_7 (Effects|SpawnEmitterAttached "/Game/Particles/MuzzleFlash_Part.MuzzleFlash_Part" (Variables|Default|GetWeapon_L) "Barrel" "0, 0, 0" "0, 0,0.000000"))
                              (Effects|Components|ParticleSystem|SetVectorParameter _returnvalue_7 "Muzzle_Color" (Math|Conversions|ToVector(LinearColor) "(R=1.000000,G=0.519954,B=0.000000,A=1.000000)"))
                              (else
                                (bind _returnvalue_8 (Effects|SpawnEmitterAttached "/Game/Particles/MuzzleFlash_Part.MuzzleFlash_Part" (Variables|Default|GetWeapon_R) "Barrel" "0, 0, 0" "0, 0,0.000000"))
                                (Effects|Components|ParticleSystem|SetVectorParameter _returnvalue_8 "Muzzle_Color" (Math|Conversions|ToVector(LinearColor) "(R=1.000000,G=0.519954,B=0.000000,A=1.000000)")))))))
                      (:then_2
                        (if _returnvalue_5
                          (bind _asdystopian_character_base (Utilities|Casting|CastToDystopianCharacterBase (.HitActor (Collision|BreakHitResult _outhit))))
                          (Class|HealthInterface|HealthInterface(Message) _asdystopian_character_base (Variables|Default|GetDamage) self)))
                      (:then_3
                        (Variables|Default|SetIsShooting? true)
                        (CallFunction|IsShooting))
                      (:then_4
                        (bind _asgatsby_anim (Utilities|Casting|CastToGatsby_Anim (Components|SkeletalMesh|GetAnimInstance (Variables|Character|GetMesh))))
                        (if (Utilities|Enum|Equal(Enum) (Variables|Default|GetWeaponType) "NewEnumerator2")
                          (Default|SniperFire _asgatsby_anim)
                          (Components|Animation|PlayAnimation (Variables|Default|GetWeapon_L) "/Game/Characters/Gatsby/Animations/Sniper.Sniper" false)
                          (else
                            (Default|FireShotgun _asgatsby_anim)
                            (Components|Animation|PlayAnimation (Variables|Default|GetWeapon_R) "/Game/Characters/Gatsby/Animations/Shotgun_mesh.Shotgun_mesh" false))))))
                  (:then_1
                    (goto _label_2))))))
          (:then_2
            (Utilities|FlowControl|Delay (Variables|Default|GetFireRate))
            (goto _label Open))
          (:then_3
            (goto _label_2 Reset))
          (:then_4
            (goto _label_3 Reset))))))
  (:Released
    (Variables|Default|SetIsShooting? false)))

(event Input|ActionEvents|InputActionMelee
  (params (Key :type Key%20Structure :default "AnyKey"))
  (:Pressed
    (Variables|Default|SetIsMeleeing true)
    (Utilities|FlowControl|Delay 0.2)))

(event Input|ActionEvents|InputActionJump
  (params (Key :type Key%20Structure :default "AnyKey"))
  ;[1 1 1] JumpLogic
  (:Pressed
    (Character|Jump))
  (:Released
    (Character|StopJumping)))

(event Input|ActionEvents|InputActionCellphone
  (params (Key :type Key%20Structure :default "AnyKey"))
  (:Pressed
    (Variables|Default|SetCellphoneEquipped? true)
    (Variables|Default|SetCanShoot false)
    (bind _returnvalue (UserInterface|CreateWidget "/Game/Interface/InGameMenu/InGameMenu_Widget.InGameMenu_Widget_C" (Game|GetPlayerController 0)))
    (UserInterface|Viewport|AddtoViewport _returnvalue 0)))

(event Input|ActionEvents|InputActionChangeView
  (params (Key :type Key%20Structure :default "AnyKey"))
  (bind _skeletalmesh (Variables|Default|GetSkeletalMesh))
  (bind _mesh (Variables|Character|GetMesh))
  (bind _weapon_r (Variables|Default|GetWeapon_R))
  (bind _fp_mesh (Variables|Default|GetFP_mesh))
  (bind _fp_camera (Variables|Default|GetFp_Camera))
  (bind _tp_camera (Variables|Default|GetTP_Camera))
  (:Pressed
    (Utilities|FlowControl|FlipFlop
      (:A
        (Class|PrimitiveComponent|SetOwnerNoSee _mesh true)
        (Class|PrimitiveComponent|SetOwnerNoSee _weapon_r true)
        (Class|PrimitiveComponent|SetOwnerNoSee _fp_mesh false)
        (Class|PrimitiveComponent|SetOwnerNoSee _skeletalmesh false)
        (Components|Activation|SetActive _fp_camera true false)
        (Components|Activation|SetActive _tp_camera false false))
      (:B
        (Class|PrimitiveComponent|SetOwnerNoSee _mesh false)
        (Class|PrimitiveComponent|SetOwnerNoSee _weapon_r false)
        (Class|PrimitiveComponent|SetOwnerNoSee _fp_mesh true)
        (Class|PrimitiveComponent|SetOwnerNoSee _skeletalmesh true)
        (Components|Activation|SetActive _fp_camera false false)
        (Components|Activation|SetActive _tp_camera true false)))))

(event Input|ActionEvents|InputActionAim
  (params (Key :type Key%20Structure :default "AnyKey"))
  (bind _charactermovement (Variables|Character|GetCharacterMovement))
  ;[1 1 1] AimLogic
  (:Pressed
    (Variables|/Script/Engine.CharacterMovementComponent|SetbUseControllerDesiredRotation _charactermovement true)
    (Variables|/Script/Engine.CharacterMovementComponent|SetbOrientRotationToMovement _charactermovement false)
    (Variables|Default|SetAiming? true))
  (:Released
    (if (== (Variables|/Script/Engine.CharacterMovementComponent|GetMaxWalkSpeed _charactermovement) (Variables|Default|GetDefaultRunSpeed))
      (Variables|/Script/Engine.CharacterMovementComponent|SetbUseControllerDesiredRotation _charactermovement false)
      (Variables|/Script/Engine.CharacterMovementComponent|SetbOrientRotationToMovement _charactermovement true)
      (Variables|Default|SetAiming? false)
      (else
        (Variables|Default|SetAiming? false)))))

(event Input|ActionEvents|InputActionSaveGame
  (params (Key :type Key%20Structure :default "AnyKey"))
  (:Pressed
    (bind _returnvalue (UserInterface|CreateWidget "/Game/Interface/InGameMenu/InGameMenu_Widget.InGameMenu_Widget_C" (Game|GetPlayerController 0)))
    (UserInterface|Viewport|AddtoViewport _returnvalue 0)))

(event Input|AxisEvents|InputAxisMoveForward
  (params (AxisValue :type Float%20%28single-precision%29))
  ;[1 1 1] KeyboardMovement
  (Pawn|Input|AddMovementInput (Math|Vector|GetForwardVector (Math|Rotator|MakeRotator 0.0 0.0 (.Yaw (Math|Rotator|BreakRotator (Pawn|GetControlRotation :!class /Script/Engine.Pawn))))) AxisValue false))

(event Input|AxisEvents|InputAxisMoveRight
  (params (AxisValue :type Float%20%28single-precision%29))
  ;[1 1 1] KeyboardMovement
  (Pawn|Input|AddMovementInput (Math|Vector|GetRightVector (Math|Rotator|MakeRotator 0.0 0.0 (.Yaw (Math|Rotator|BreakRotator (Pawn|GetControlRotation :!class /Script/Engine.Pawn))))) AxisValue false))

(event Input|AxisEvents|InputAxisLookUp
  (params (AxisValue :type Float%20%28single-precision%29))
  (bind _returnvalue (Pawn|GetControlRotation :!class /Script/Engine.Pawn))
  (bind _returnvalue_2 (Pawn|GetController))
  (bind (_roll _pitch _yaw) (Math|Rotator|BreakRotator _returnvalue))
  ;[1 1 1] MouseInput
  (Utilities|IsValid _returnvalue_2
    (:Is%20Valid
      (Pawn|SetControlRotation _returnvalue_2 (Math|Rotator|MakeRotator _roll (Math|Float|ClampAngle (+ (* AxisValue -1.0) _pitch) -8e+01 9e+01) _yaw)))))

(event Input|AxisEvents|InputAxisTurn
  (params (AxisValue :type Float%20%28single-precision%29))
  ;[1 1 1] MouseInput
  (Utilities|FlowControl|Sequence
    (:then_0
      (Pawn|Input|AddControllerYawInput AxisValue))
    (:then_1
      (if (Math|Vector|Equal(Vector) (Transformation|GetVelocity) "0, 0, 0" 0.0001)
        (Utilities|FlowControl|Sequence
          (:then_0
            (if (> AxisValue 0.03)
              (Variables|Default|SetTurnRight true)
              (Variables|Default|SetTurnLeft false)
              (else
                (Variables|Default|SetTurnRight false))))
          (:then_1
            (if (< AxisValue -0.03)
              (Variables|Default|SetTurnLeft true)
              (else
                (Variables|Default|SetTurnLeft false)))))))))

(event Input|KeyboardEvents|3
  (params (Key :type Key%20Structure :default "AnyKey"))
  (:Pressed
    (Variables|Default|SetDamage 2e+03)))

(event Input|KeyboardEvents|K
  (params (Key :type Key%20Structure :default "AnyKey"))
  (:Pressed
    (CallFunction|HealthInterface 1.0)))

(event Input|KeyboardEvents|L
  (params (Key :type Key%20Structure :default "AnyKey"))
  (:Pressed
    (CallFunction|HealthInterface -1e+03)))

(fn ConstructionScript)

(fn WeaponVariables
  (params (NewParam :type Gatsby%20Weapon%20Struc%20Structure))
  (bind (_damage _firerate _weaponspread _burstcount _attackrange _reloadspeed _maxammo _weaponname _weapontype _ammotype _lefthanded_ _weaponmesh) (Utilities|Struct|BreakGatsby_WeaponStruc NewParam))
  (bind _weapon_r (Variables|Default|GetWeapon_R))
  (bind _weapon_l (Variables|Default|GetWeapon_L))
  (Variables|Default|SetDamage _damage)
  (Variables|Default|SetFireRate _firerate)
  (Variables|Default|SetWeaponSpread _weaponspread)
  (Variables|Default|SetBurstCount _burstcount)
  (Variables|Default|SetAttackRange _attackrange)
  (Variables|Default|SetReloadSpeed _reloadspeed)
  (Variables|Default|SetMaxAmmo _maxammo)
  (Variables|Default|SetWeaponName _weaponname)
  (Variables|Default|SetWeaponType _weapontype)
  (Variables|Default|SetAmmoType _ammotype)
  (Variables|Default|SetLeftHanded? _lefthanded_)
  (if _lefthanded_
    (Class|SkinnedMeshComponent|SetSkeletalMesh _weapon_l _weaponmesh true)
    (Class|SkinnedMeshComponent|SetSkeletalMesh _weapon_r 0 true)
    (else
      (Class|SkinnedMeshComponent|SetSkeletalMesh _weapon_l 0 true)
      (Class|SkinnedMeshComponent|SetSkeletalMesh _weapon_r _weaponmesh true))))