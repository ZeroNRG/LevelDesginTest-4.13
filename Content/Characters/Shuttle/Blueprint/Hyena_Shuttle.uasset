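; Hyena dropship pawn that delivers two Hyena characters, then flies away and destroys itself.
; On BeginPlay it plays a hover animation, spawns both passengers attached to mesh sockets, and plays their idle then staggered exit animations.
; Each surviving passenger gets an AI controller, detaches and has its roll zeroed.
; Timed delays drive the sequence; the shuttle then switches to its AnimBP and moves to a hardcoded point without pathfinding.
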(event EventBeginPlay
  (Pawn|SpawnDefaultController)
  (Utilities|FlowControl|Sequence
    (:then_0
      (Components|Animation|PlayAnimation (Variables|Character|GetMesh) "/Game/Characters/Shuttle/Animation/Dropship_ShuttleHover.Dropship_ShuttleHover" false))
    (:then_1
      (Utilities|FlowControl|Sequence
        (:then_0
          (bind _returnvalue (Game|SpawnActorfromClass "/Game/Characters/Hyena/Blueprint/Hyena_Chara.Hyena_Chara_C" (Math|Transform|MakeTransform "0, 0,0.000000" "0,0.000000,0.000000") "AlwaysSpawn" 0 0))
          (Variables|/Game/Characters/Hyena/Blueprint/Hyena_Chara.Hyena_Chara_C|SetShuttleSpawn _returnvalue true)
          (Transformation|AttachComponentToComponent (Variables|/Script/Engine.Character|GetCapsuleComponent _returnvalue) (Variables|Character|GetMesh) "P2Socket" "KeepRelative" "KeepRelative" "KeepRelative" false)
          (Components|Animation|PlayAnimation (Variables|/Script/Engine.Character|GetMesh _returnvalue) "/Game/Characters/Hyena/Animation/Hyena_Dropship_DropShip_Idle.Hyena_Dropship_DropShip_Idle" true)
          (Utilities|FlowControl|Delay 2.0)
          (Components|Animation|PlayAnimation (Variables|/Script/Engine.Character|GetMesh _returnvalue) "/Game/Characters/Hyena/Animation/Hyena_Dropship_DropShip_Exit.Hyena_Dropship_DropShip_Exit" false)
          (Utilities|FlowControl|Delay 1.7)
          (Utilities|IsValid _returnvalue
            (:Is%20Valid
              (Pawn|SpawnDefaultController _returnvalue)
              (Transformation|DetachFromComponent (Variables|/Script/Engine.Character|GetCapsuleComponent _returnvalue) "KeepWorld" "KeepWorld" "KeepWorld" true)
              (Transformation|SetWorldRotation (Variables|/Script/Engine.Character|GetCapsuleComponent _returnvalue) (Math|Rotator|MakeRotator 0.0 (.Pitch (Math|Rotator|BreakRotator (Transformation|GetWorldRotation (Variables|/Script/Engine.Character|GetCapsuleComponent _returnvalue)))) (.Yaw (Math|Rotator|BreakRotator (Transformation|GetWorldRotation (Variables|/Script/Engine.Character|GetCapsuleComponent _returnvalue))))) false false))))
        (:then_1
          (bind _returnvalue_2 (Game|SpawnActorfromClass "/Game/Characters/Hyena/Blueprint/Hyena_Chara.Hyena_Chara_C" (Math|Transform|MakeTransform "0, 0,0.000000" "0,0.000000, 0") "AlwaysSpawn" 0 0))
          (Variables|/Game/Characters/Hyena/Blueprint/Hyena_Chara.Hyena_Chara_C|SetShuttleSpawn _returnvalue_2 true)
          (Transformation|AttachComponentToComponent (Variables|/Script/Engine.Character|GetCapsuleComponent _returnvalue_2) (Variables|Character|GetMesh) "P1Socket" "KeepRelative" "KeepRelative" "KeepRelative" true)
          (Components|Animation|PlayAnimation (Variables|/Script/Engine.Character|GetMesh _returnvalue_2) "/Game/Characters/Hyena/Animation/Hyena_Dropship_DropShip_Idle.Hyena_Dropship_DropShip_Idle" true)
          (Utilities|FlowControl|Delay 1.5)
          (Components|Animation|PlayAnimation (Variables|/Script/Engine.Character|GetMesh _returnvalue_2) "/Game/Characters/Hyena/Animation/Hyena_Dropship_DropShip_Exit.Hyena_Dropship_DropShip_Exit" false)
          (Utilities|FlowControl|Delay 1.7)
          (Utilities|IsValid _returnvalue_2
            (:Is%20Valid
              (Pawn|SpawnDefaultController _returnvalue_2)
              (Transformation|DetachFromComponent (Variables|/Script/Engine.Character|GetCapsuleComponent _returnvalue_2) "KeepWorld" "KeepWorld" "KeepWorld" true)
              (Transformation|SetWorldRotation (Variables|/Script/Engine.Character|GetCapsuleComponent _returnvalue_2) (Math|Rotator|MakeRotator 0.0 (.Pitch (Math|Rotator|BreakRotator (Transformation|GetWorldRotation (Variables|/Script/Engine.Character|GetCapsuleComponent _returnvalue_2)))) (.Yaw (Math|Rotator|BreakRotator (Transformation|GetWorldRotation (Variables|/Script/Engine.Character|GetCapsuleComponent _returnvalue_2))))) false false))))))
    (:then_2
      (bind _returnvalue_3 (AI|GetAIController self))
      (Utilities|FlowControl|Delay 4.7)
      (Components|Animation|SetAnimationMode (Variables|Character|GetMesh) "AnimationBlueprint")
      (AI|Navigation|MovetoLocation _returnvalue_3 (Math|Vector|MakeVector -6.8e+02 -1.615e+04 5e+03) -1.0 true false false false)
      (Utilities|FlowControl|Delay 1e+01)
      (Actor|DestroyActor))))

(fn ConstructionScript)