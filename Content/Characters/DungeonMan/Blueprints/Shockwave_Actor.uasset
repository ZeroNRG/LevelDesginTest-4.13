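; Shockwave actor for DungeonMan that expands and damages characters it touches, then destroys itself.
; A timeline scales the static mesh on BeginPlay, with separate curves for horizontal size and height.
; Mesh overlap and hit events both run a cast to DystopianCharacterBase and send fixed damage through its health interface.
; Disconnected leftovers include a height-checked sphere trace damage path and once-only gating.
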(event OnComponentBeginOverlap(StaticMesh)
  (params (OverlappedComponent :type Primitive%20Component%20Object%20Reference) (OtherActor :type Actor%20Object%20Reference) (OtherComp :type Primitive%20Component%20Object%20Reference) (OtherBodyIndex :type Integer) (bFromSweep :type Boolean) (SweepResult :type Hit%20Result%20Structure%20%28by%20ref%29))
  (bind _asdystopian_character_base (Utilities|Casting|CastToDystopianCharacterBase OtherActor))
  (Default|HealthInterface _asdystopian_character_base 15.0 self "None"))

(event OnComponentHit(StaticMesh)
  (params (HitComponent :type Primitive%20Component%20Object%20Reference) (OtherActor :type Actor%20Object%20Reference) (OtherComp :type Primitive%20Component%20Object%20Reference) (NormalImpulse :type Vector :default "0, 0, 0") (Hit :type Hit%20Result%20Structure%20%28by%20ref%29))
  (bind _asdystopian_character_base (Utilities|Casting|CastToDystopianCharacterBase (stale OnComponentBeginOverlap(StaticMesh) OtherActor)))
  (Default|HealthInterface _asdystopian_character_base 15.0 self "None"))

(event EventBeginPlay
  (bind (_direction _scale _zscale) (Timeline|Shockwave%20scale Play)
    (:Update
      (Transformation|SetRelativeScale3D (Variables|Default|GetStaticMesh) (Math|Vector|MakeVector _scale _scale _zscale)))
    (:Finished
      (Actor|DestroyActor))))

(event EventTick
  (params (DeltaSeconds :type Float%20%28single-precision%29)))

(fn ConstructionScript)