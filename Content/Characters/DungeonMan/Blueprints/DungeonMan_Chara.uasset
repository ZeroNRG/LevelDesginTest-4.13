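; DungeonMan character Blueprint that turns to face its target, fires ground shockwaves and plays a death animation.
; Tick eases yaw toward TargetActor and updates TurnLeft from the yaw delta, clearing it only at exactly zero.
; Ground_Fire spawns a Shockwave_Actor at each of the left and right barrel sockets.
; BeginPlay binds the death event that plays the death animation; a camera-facing StaticMesh rotation is left unconnected.
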(event Custom|Ground_Fire
  (bind _mesh (Variables|Character|GetMesh))
  (bind _mesh_2 (Variables|Character|GetMesh))
  (bind _returnvalue (Transformation|GetSocketTransform _mesh_2 "Barrel_L" "RTS_World"))
  (bind _returnvalue_2 (Transformation|GetSocketTransform _mesh "Barrel_R" "RTS_World"))
  (bind (_location _rotation _scale) (Math|Transform|BreakTransform _returnvalue_2))
  (bind (_location_2 _rotation_2 _scale_2) (Math|Transform|BreakTransform _returnvalue))
  (Game|SpawnActorfromClass "/Game/Characters/DungeonMan/Blueprints/Shockwave_Actor.Shockwave_Actor_C" (Math|Transform|MakeTransform _location_2 "0, 0, 0" _scale_2) "Undefined" 0 0)
  (Game|SpawnActorfromClass "/Game/Characters/DungeonMan/Blueprints/Shockwave_Actor.Shockwave_Actor_C" (Math|Transform|MakeTransform _location "0, 0, 0" _scale) "Undefined" 0 0))

(event Custom|DeathAnim
  (Components|Animation|PlayAnimation (Variables|Character|GetMesh) "/Game/Characters/DungeonMan/Animation/DungeonMan_Death.DungeonMan_Death" false))

(event Collision|EventActorBeginOverlap
  (params (OtherActor :type Actor%20Object%20Reference)))

(event EventBeginPlay
  (EventDispatchers|BindEventtoDeathAnimation (delegate Custom|DeathAnim)))

(event EventTick
  (params (DeltaSeconds :type Float%20%28single-precision%29))
  (bind _returnvalue (Transformation|GetActorLocation))
  (bind _returnvalue_2 (Transformation|GetActorRotation))
  (bind _targetactor (Variables|Default|GetTargetActor))
  (bind _returnvalue_3 (Transformation|GetActorLocation _targetactor))
  (bind _returnvalue_4 (Math|Rotator|FindLookatRotation _returnvalue _returnvalue_3))
  (bind _yaw (Math|Rotator|BreakRotator _returnvalue_4))
  (bind _returnvalue_5 (Math|Rotator|MakeRotator 0.0 0.0 _yaw))
  (bind _returnvalue_6 (Math|Rotator|Delta(Rotator) _returnvalue_2 _returnvalue_5))
  (bind _yaw_2 (Math|Rotator|BreakRotator _returnvalue_6))
  (Utilities|IsValid _targetactor
    (:Is%20Valid
      (Transformation|SetActorRotation (Math|Interpolation|RInterpTo _returnvalue_2 _returnvalue_5 (Utilities|Time|GetWorldDeltaSeconds) 1.0))
      (if (> _yaw_2 0.0)
        (Variables|Default|SetTurnLeft true)
        (elif (not (< _yaw_2 0.0))
          (Variables|Default|SetTurnLeft false))))))

(fn ConstructionScript)