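; Car prop Blueprint that tints its static mesh with a configurable body color.
; On BeginPlay it converts the CarColor variable to a vector and writes it to the CarDiffuse parameter on the mesh's materials.
; A random pick from a four-color palette is present but unconnected, and the construction script is empty, so the tint is applied only at runtime.
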(event EventBeginPlay
  (Rendering|Material|SetVectorParameterValueonMaterials (Variables|Default|GetStaticMesh) "CarDiffuse" (Math|Conversions|ToVector(LinearColor) (Variables|Default|GetCarColor))))

(event Collision|EventActorBeginOverlap
  (params (OtherActor :type Actor%20Object%20Reference)))

(event EventTick
  (params (DeltaSeconds :type Float%20%28single-precision%29)))

(fn ConstructionScript)